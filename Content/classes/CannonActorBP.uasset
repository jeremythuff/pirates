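; CannonActorBP is a cannon actor that turns its sprite to face whatever enters its range.
; Overlap events on the CannonRange component store the entering actor as Target and toggle IsTracking on entry and exit.
; Each Tick, UpdateCannonAim applies only the look-at yaw toward Target, taking roll and pitch from the sprite's relative rotation.
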(event OnComponentBeginOverlap(CannonRange)
  (params (OverlappedComponent :type Primitive%20Component%20Object%20Reference) (OtherActor :type Actor%20Object%20Reference) (OtherComp :type Primitive%20Component%20Object%20Reference) (OtherBodyIndex :type Integer) (bFromSweep :type Boolean) (SweepResult :type Hit%20Result%20Structure%20%28by%20ref%29))
  ;[1 1 1] Enter cannon range
  (Variables|Default|SetTarget OtherActor)
  (Variables|Default|SetIsTracking true))

(event OnComponentEndOverlap(CannonRange)
  (params (OverlappedComponent :type Primitive%20Component%20Object%20Reference) (OtherActor :type Actor%20Object%20Reference) (OtherComp :type Primitive%20Component%20Object%20Reference) (OtherBodyIndex :type Integer))
  ;[1 1 1] Leave cannon range
  (Variables|Default|SetIsTracking false))

(event Custom|Update%20Cannon%20Aim
  (bind _cannonsprite (Variables|Default|GetCannonSprite))
  (bind _relativerotation (Variables|/Script/Engine.SceneComponent|GetRelativeRotation _cannonsprite))
  (bind (_roll _pitch) (Math|Rotator|BreakRotator _relativerotation))
  (if (Variables|Default|GetIsTracking)
    (Transformation|SetWorldRotation (Variables|Default|GetCannonSprite) (Math|Rotator|MakeRotator _roll _pitch (.Yaw (Math|Rotator|BreakRotator (Math|Rotator|FindLookatRotation (Transformation|GetWorldLocation _cannonsprite) (Transformation|GetActorLocation (Variables|Default|GetTarget)))))) false false)))

(event EventBeginPlay)

(event Collision|EventActorBeginOverlap
  (params (OtherActor :type Actor%20Object%20Reference)))

(event EventTick
  (params (DeltaSeconds :type Float%20%28single-precision%29))
  (CallFunction|UpdateCannonAim))

(fn ConstructionScript)