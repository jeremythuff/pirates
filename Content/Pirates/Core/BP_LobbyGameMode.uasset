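; Lobby game mode for the Pirates game that registers joining players, sends them lobby settings and spawns each as a base ship at a random PlayerStart.
; EveryoneUpdate refreshes every controller's player list, count and teams, and flags readiness false if any ship is still the base one.
; LaunchTheGame server-travels to one of two arenas by map ID.
; Ship swapping and kick listing are empty stubs, and map changes are stored but not broadcast.
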(event Custom|SwapShip
  (params (PlayerController :type Player%20Controller%20Object%20Reference) (ShipClass :type Ship%20Base%20BP%20Class%20Reference) (ChangedStatus :type Boolean)))

(event Custom|LaunchTheGame
  (bind _returnvalue (Game|GetPlayerController 0))
  (switch int (Variables|ServerSettings|GetGMMapID)
    (:0
      (Development|ExecuteConsoleCommand "servertravel /Games/Maps/Arena01" _returnvalue))
    (:1
      (Development|ExecuteConsoleCommand "servertravel /Games/Maps/Arena02" _returnvalue))))

(event Custom|RespawnPlayer
  (params (PlayerController :type BP%20Lobby%20Player%20Controller%20Object%20Reference))
  (bind _returnvalue (Pawn|GetControlledPawn PlayerController))
  (bind _spawn_points (Variables|ServerSettings|GetSpawn%20Points))
  ;[1 1 1] Spawn a charachter as base character when arriving at the lobby
  (Utilities|IsValid _returnvalue
    (:Is%20Valid
      (Actor|DestroyActor _returnvalue))
    (:Is%20Not%20Valid
      _))
  (bind _returnvalue_2 (Game|SpawnActorfromClass "/Game/Blueprints/Ship/ShipBaseBP.ShipBaseBP_C" (Transformation|GetActorTransform (Utilities|Array|Get(acopy) _spawn_points (Math|Random|RandomIntegerinRange 0 (- (Utilities|Array|Length _spawn_points) 1)))) "Undefined" 0 0))
  (Pawn|Possess PlayerController _returnvalue_2)
  (CallFunction|EveryoneUpdate))

(event Custom|EveryoneUpdate
  (bind _allplayercontrollers (Variables|ServerSettings|GetAllPlayerControllers))
  (bind _allplayercontrollers_2 (Variables|ServerSettings|GetAllPlayerControllers))
  (bind _returnvalue (Utilities|Array|Length _allplayercontrollers))
  ;[1 1 1] Update All Connected players' lobby info
  (Variables|ServerSettings|SetCurrentPlayers _returnvalue)
  (if (> _returnvalue 0)
    (Utilities|Array|Clear (Variables|ServerSettings|GetConnectedPlayers))
    (for _array_element _allplayercontrollers_2
      (Utilities|Array|Add (Variables|ServerSettings|GetConnectedPlayers) (Variables|/Game/Pirates/Core/BP_LobbyPlayerController.BP_LobbyPlayerController_C|GetPlayer%20Settings _array_element))
      (Default|UpdateNumberOfPlayers _array_element (Variables|ServerSettings|GetCurrentPlayers) (Variables|ServerSettings|GetMax%20Players)))
    (for _array_element_2 _allplayercontrollers_2
      (Default|AddPlayerInfo _array_element_2 (Variables|ServerSettings|GetConnectedPlayers))
      (Default|UpdateAvailableTeams _array_element_2 (Variables|ServerSettings|GetAvailable%20Teams))
      (CallFunction|AddtoKickList))
    (bind _array_element_3 (Utilities|Array|ForEachLoopwithBreak (Variables|ServerSettings|GetConnectedPlayers))
      (:LoopBody
        (if (== (.PiratesPlayerShip (Utilities|Struct|BreakSPiratesPlayerInfo _array_element_3)) "/Game/Blueprints/Ship/ShipBaseBP.ShipBaseBP_C")
          (Variables|ServerSettings|SetisReadyToStart false)
          (CallFunction|CannotStart)
          (else
            (Variables|ServerSettings|SetisReadyToStart true)))))))

(event Custom|AddToKickList)

(event Custom|Cannot%20Start
  ;[1 1 1] Update All Connected players' lobby info
  (Utilities|Array|ForEachLoopwithBreak (Variables|ServerSettings|GetConnectedPlayers)) ; enters at Break
)

(event Custom|ServerUdateGameSettings
  (params (MapImage :type Texture%202D%20Object%20Reference) (MapName :type Text) (MapTime :type Text) (MapID :type Integer))
  ;[1 1 1] Server has made changes
  (Variables|ServerSettings|SetGMMapImage MapImage)
  (Variables|ServerSettings|SetGMMapName MapName)
  (Variables|ServerSettings|SetGMMapTime MapTime)
  (Variables|ServerSettings|SetGMMapID MapID)
  (for _array_element (Variables|ServerSettings|GetAllPlayerControllers)
    _))

(event EventPostLogin
  (params (NewPlayer :type Player%20Controller%20Object%20Reference))
  (bind _returnvalue (Game|GetGameInstance))
  (bind _asbp_pirates_game_instance (Utilities|Casting|CastToBP_PiratesGameInstance _returnvalue))
  ;[1 1 1] Initial Setup
  (bind _asbp_lobby_player_controller (Utilities|Casting|CastToBP_LobbyPlayerController NewPlayer))
  (Networking|SwitchHasAuthority
    (:Authority
      (Utilities|Array|Add (Variables|ServerSettings|GetAllPlayerControllers) _asbp_lobby_player_controller)
      (bind _outactors (Actor|GetAllActorsOfClass "/Script/Engine.PlayerStart"))
      (Variables|ServerSettings|SetSpawn%20Points _outactors)
      (bind _output_get (Variables|ServerSettings|SetServer%20Name (Variables|/Game/Pirates/Core/BP_PiratesGameInstance.BP_PiratesGameInstance_C|GetServer%20Name _asbp_pirates_game_instance)))
      (Variables|ServerSettings|SetMax%20Players (Variables|/Game/Pirates/Core/BP_PiratesGameInstance.BP_PiratesGameInstance_C|GetMax%20Players _asbp_pirates_game_instance))
      (Default|InitialSetup _asbp_lobby_player_controller)
      (Default|SetupLobbyMenu _asbp_lobby_player_controller (Utilities|Text|ToText(String) _output_get))
      (Default|UpdateLobbySettings _asbp_lobby_player_controller (Variables|ServerSettings|GetGMMapImage) (Variables|ServerSettings|GetGMMapName) (Variables|ServerSettings|GetGMMapTime))
      (CallFunction|RespawnPlayer _asbp_lobby_player_controller))))

(fn ConstructionScript)