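; Base ship Blueprint that plays motion-based water effects and fires a cannon.
; Each Tick it checks velocity, switching the ShipRipple flipbook between Wake and Ripple and fading the movement sound in or out.
; Releasing Space Bar spawns a cannonball at the CannonPort's Barrel socket and plays the shot sound at the world origin rather than at the ship.
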(event Custom|Update%20Animation
  (bind _moving_sound (Variables|Default|GetMoving%20Sound))
  (bind _returnvalue (Audio|Components|Audio|IsPlaying _moving_sound))
  ;[1 1 1] Change the Animation of the ship from idle to in motion
  (if (> (Math|Vector|VectorLength (Transformation|GetVelocity)) 0.0)
    (if _returnvalue
      _
      (else
        (Audio|Components|Audio|FadeIn _moving_sound 1.0 0.85 0.0 :!class /Script/Engine.AudioComponent)))
    (Variables|Default|SetCurrent%20Animation "/Game/sprite_flipbooks/wake.wake")
    (else
      (if _returnvalue
        (Audio|Components|Audio|FadeOut _moving_sound 1.0 0.0 :!class /Script/Engine.AudioComponent))
      (Variables|Default|SetCurrent%20Animation "/Game/sprite_flipbooks/ripple.ripple")))
  (Sprite|SetFlipbook (Variables|Default|GetShipRipple) (Variables|Default|GetCurrent%20Animation)))

(event EventBeginPlay)

(event Collision|EventActorBeginOverlap
  (params (OtherActor :type Actor%20Object%20Reference)))

(event EventTick
  (params (DeltaSeconds :type Float%20%28single-precision%29))
  (CallFunction|UpdateAnimation))

(event Input|KeyboardEvents|SpaceBar
  (params (Key :type Key%20Structure))
  ;[1 1 1] Fire the cannon
  (:Released
    (Game|SpawnActorfromClass "/Game/blueprints/Cannon/CannonBallActoprBP.CannonBallActoprBP_C" (Transformation|GetSocketTransform (Variables|Default|GetCannon%20Port) "Barrel" "RTS_World") "Undefined" self 0)
    (Audio|PlaySoundatLocation "/Game/audio/cannonshot.cannonshot" "0, 0, 0")))

(fn ConstructionScript)