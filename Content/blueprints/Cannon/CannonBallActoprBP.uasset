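; Paper2D cannonball projectile actor owned by a CannonActorBP, which hits targets and explodes.
; On collision with an actor implementing the Hitable interface, it sends HitMessage once, guarded by IsBeingHit, and triggers destruction.
; Every tick it also triggers destruction if its horizontal distance from the cannon exceeds that cannon's Range.
; Destruction clears the sprite, sets a non-looping strike flipbook and destroys the actor after the animation's length.
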(event OnComponentHit(CannonBallCollision)
  (params (HitComponent :type Primitive%20Component%20Object%20Reference) (OtherActor :type Actor%20Object%20Reference) (OtherComp :type Primitive%20Component%20Object%20Reference) (NormalImpulse :type Vector :default "0, 0, 0") (Hit :type Hit%20Result%20Structure%20%28by%20ref%29))
  ;[1 1 1] Fire cannon ball, display explosion and destroy cannon ball
  (if (Utilities|DoesObjectImplementInterface OtherActor "/Script/pirates.Hitable")
    (if (Math|Boolean|NotEqual(Boolean) (Variables|Default|GetIsBeingHit) true)
      (Variables|Default|SetIsBeingHit true)
      (Class|Hitable|Hit(Message) OtherActor)
      (CallFunction|DestroyCannonball))))

(event Custom|Destroy%20Cannonball
  (bind _cannonballexplosion (Variables|Default|GetCannonBallExplosion))
  ;[1 1 1] Destroy Cannonball
  (Components|Timeline|SetLooping _cannonballexplosion false)
  (Sprite|SetFlipbook _cannonballexplosion "/Game/sprite_flipbooks/cannon_strike.cannon_strike")
  (Rendering|Components|Sprite|SetSprite (Variables|Default|GetCannonBallSprite) 0)
  (Utilities|FlowControl|Delay (Class|PaperFlipbookComponent|GetFlipbookLength (Variables|Default|GetCannonBallExplosion)))
  (Actor|DestroyActor))

(event Custom|Check%20Distance%20Traveled
  (bind _cannon (Variables|Default|GetCannon))
  ;[1 1 1] Check distance the cannonball has travelled
  (if (> (Math|Vector|VectorLengthXY (- (Transformation|GetActorLocation) (Transformation|GetActorLocation _cannon))) (Variables|/Game/blueprints/Cannon/CannonActorBP.CannonActorBP_C|GetRange _cannon))
    (CallFunction|DestroyCannonball)))

(event EventBeginPlay
  (bind _ascannon_actor_bp (Utilities|Casting|CastToCannonActorBP (Components|GetOwner)))
  (Variables|Default|SetCannon _ascannon_actor_bp))

(event Collision|EventActorBeginOverlap
  (params (OtherActor :type Actor%20Object%20Reference)))

(event EventTick
  (params (DeltaSeconds :type Float%20%28single-precision%29))
  (CallFunction|CheckDistanceTraveled))

(fn ConstructionScript)