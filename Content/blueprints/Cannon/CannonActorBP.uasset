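; Auto-targeting cannon actor that fires cannonballs at Hitable actors within its capsule range.
; Range overlaps maintain a target list, from which it picks the nearest in XY only when the current target is invalid.
; Tick smoothly turns it toward the target and calls fire, where a Delay throttles shots.
; Shots spawn at the sprite's Barrel socket with a sound while target HP is positive; otherwise the target leaves the list.
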(event OnComponentEndOverlap(CannonRange)
  (params (OverlappedComponent :type Primitive%20Component%20Object%20Reference) (OtherActor :type Actor%20Object%20Reference) (OtherComp :type Primitive%20Component%20Object%20Reference) (OtherBodyIndex :type Integer))
  ;[1 1 1] When actor leaves range remove from targets
  (Utilities|Array|RemoveItem (Variables|Default|GetTargets) OtherActor))

(event OnComponentBeginOverlap(CannonRange)
  (params (OverlappedComponent :type Primitive%20Component%20Object%20Reference) (OtherActor :type Actor%20Object%20Reference) (OtherComp :type Primitive%20Component%20Object%20Reference) (OtherBodyIndex :type Integer) (bFromSweep :type Boolean) (SweepResult :type Hit%20Result%20Structure%20%28by%20ref%29))
  ;[1 1 1] When actor overlaps range add to targets
  (if (Utilities|DoesObjectImplementInterface OtherActor "/Script/pirates.Hitable")
    (Utilities|Array|Add (Variables|Default|GetTargets) OtherActor)))

(event Custom|CannonFire
  (bind _target (Variables|Default|GetTarget))
  ;[1 1 1] Fire the cannon
  (Utilities|FlowControl|Delay 2.0)
  (Utilities|IsValid _target
    (:Is%20Valid
      (bind _returnvalue (Class|Hitable|GetHP(Message) _target))
      (if (> _returnvalue 0)
        (Game|SpawnActorfromClass "/Game/blueprints/Cannon/CannonBallActoprBP.CannonBallActoprBP_C" (Transformation|GetSocketTransform (Variables|Default|GetCannonSprite) "Barrel" "RTS_World") "Undefined" self 0)
        (Audio|PlaySoundatLocation "/Game/blueprints/sounds/CannonFire.CannonFire" "0, 0, 0")
        (else
          (Utilities|Array|RemoveItem (Variables|Default|GetTargets) _target))))))

(event Custom|Aim%20Cannon
  ;[1 1 1] Change cannon rotation to match target
  (if (> (Utilities|Array|Length (Variables|Default|GetTargets)) 0)
    (Utilities|IsValid (Variables|Default|GetTarget)
      (:Is%20Valid
        _)
      (:Is%20Not%20Valid
        (CallFunction|SelectTarget)))
    (Transformation|SetActorRotation (Math|Interpolation|RInterpTo (Transformation|GetActorRotation) (Math|Rotator|FindLookatRotation (Transformation|GetActorLocation) (Transformation|GetActorLocation (Variables|Default|GetTarget))) (Variables|Default|GetDeltaTime) 5.0))
    (else
      (Variables|Default|SetTarget 0))))

(event Custom|Select%20Target
  (bind _returnvalue (Transformation|GetActorLocation))
  ;[1 1 1] Select a target from targets based on nearness to cannon
  (for _array_element (Variables|Default|GetTargets)
    (Utilities|IsValid 0
      (:Is%20Valid
        _)
      (:Is%20Not%20Valid
        (Variables|Default|SetTarget _array_element)))
    (if (< (Math|Vector|VectorLengthXY (- (Transformation|GetActorLocation _array_element) _returnvalue)) (Math|Vector|VectorLengthXY (- (Transformation|GetActorLocation (Variables|Default|GetTarget)) _returnvalue)))
      (Variables|Default|SetTarget _array_element))))

(event EventBeginPlay
  (Variables|Default|SetRange (.OutRadius (Components|Capsule|GetScaledCapsuleSize (Variables|Default|GetCannonRange)))))

(event Collision|EventActorBeginOverlap
  (params (OtherActor :type Actor%20Object%20Reference)))

(event EventTick
  (params (DeltaSeconds :type Float%20%28single-precision%29))
  ;[1 1 1] Event Tick
  (Utilities|FlowControl|Sequence
    (:then_0
      (Variables|Default|SetDeltaTime DeltaSeconds))
    (:then_1
      (CallFunction|AimCannon))
    (:then_2
      (CallFunction|CannonFire))))

(fn ConstructionScript)